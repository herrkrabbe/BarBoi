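; BP_Astronaut is the player astronaut Blueprint, handling HUD, health and a death menu.
; BeginPlay hides the mesh from its owner and creates crosshair and main widgets.
; Damage reduces Health and only prints "Game Lost" at zero; a separate OnDeath event shows the death menu and pauses the game.
; The droid switch only casts the result of GetDroid, as its Possess call is disconnected.
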(event Custom|Switch_1
  ;[1 1 1] Switch between Astronaut and Droid
  (bind _returnvalue (Class|Switch|GetDroid))
  (bind _asdroid (Utilities|Casting|CastToDroid (Utilities|ToObject(Interface) _returnvalue))
    (:CastFailed
      (Development|PrintString "Cast to droid failed"))))

(event EventBeginPlay
  ;[1 1 1] Widget for Player
  (bind _returnvalue (UserInterface|CreateWidget "/Game/Group_11/HUD/WBP_Crosshair.WBP_Crosshair_C"))
  (UserInterface|Viewport|AddtoViewport _returnvalue 0)
  (Class|PrimitiveComponent|SetOwnerNoSee (Variables|Character|GetMesh) true)
  (bind _asplayer_controller (Utilities|Casting|CastToPlayerController (Pawn|GetController self)))
  (bind _returnvalue_2 (UserInterface|CreateWidget "/Game/Group_11/HUD/WBP_MainWidget.WBP_MainWidget_C" _asplayer_controller))
  (UserInterface|Viewport|AddtoPlayerScreen _returnvalue_2))

(event EventOnDeath
  (bind _returnvalue (Game|GetPlayerController 0))
  ;[1 1 1] Death Menu
  (Variables|/Script/Engine.PlayerController|SetbShowMouseCursor _returnvalue true)
  (bind _returnvalue_2 (UserInterface|CreateWidget "/Game/Group_11/HUD/WBP_DeathMenu.WBP_DeathMenu_C"))
  (bind _output_get (Variables|Default|SetDeathMenuREF _returnvalue_2))
  (UserInterface|Viewport|AddtoViewport _output_get 0)
  (Input|SetInputModeGameandUI _returnvalue _output_get "DoNotLock" true false)
  (Game|SetGamePaused true))

(event Game|Damage|EventAnyDamage
  (params (Damage :type Float%20%28single-precision%29) (DamageType :type Damage%20Type%20Object%20Reference) (InstigatedBy :type Controller%20Object%20Reference) (DamageCauser :type Actor%20Object%20Reference))
  ;[1 1 1] Makes Astronaut take Damage
  (bind _output_get (Variables|Default|SetHealth (- (Variables|Default|GetHealth) Damage)))
  (Development|PrintString (Utilities|String|ToString(Float) _output_get))
  (if (<= (Variables|Default|GetHealth) 0.0)
    (Development|PrintString "Game Lost")))

(fn ConstructionScript)