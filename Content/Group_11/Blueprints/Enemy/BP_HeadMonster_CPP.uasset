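; BP_HeadMonster_CPP is a head monster enemy that deals contact damage to the astronaut character.
; On BeginPlay it caches its health bar widget and copies current and max health into it.
; A timer counts down on Tick, and an overlap beginning on the damage collision damages BP_Astronaut only when that timer has run out, then resets it to the attack rate.
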(event OnComponentBeginOverlap(DamageCollision)
  (params (OverlappedComponent :type Primitive%20Component%20Object%20Reference) (OtherActor :type Actor%20Object%20Reference) (OtherComp :type Primitive%20Component%20Object%20Reference) (OtherBodyIndex :type Integer) (bFromSweep :type Boolean) (SweepResult :type Hit%20Result%20Structure%20%28by%20ref%29))
  ;[1 1 1] Enemy Can Deal Damage
  (bind _asbp_astronaut (Utilities|Casting|CastToBP_Astronaut OtherActor))
  (if (<= (Variables|Default|GetAttack%20Timer) 0.0)
    (Class|Astronaut|DamageThis _asbp_astronaut (Variables|Default|GetDamage))
    (Variables|Default|SetAttack%20Timer (Variables|Default|GetAttackRate))))

(event EventBeginPlay
  ;[1 1 1] Sets Health bar on enemy
  (bind _aswp_enemy_health (Utilities|Casting|CastTo (UserInterface|GetUserWidgetObject (Variables|Default|GetWidget))))
  (bind _output_get (Variables|Default|SetWP%20Enemy%20Health _aswp_enemy_health))
  (Variables|Default|SetCurrentHealth _output_get (Variables|Default|GetCurrentHealth))
  (Variables|Default|SetMaxHealth _output_get (Variables|Default|GetMaxHealth)))

(event EventTick
  (params (DeltaSeconds :type Float%20%28single-precision%29))
  ;[1 1 1] Enemy Can Deal Damage
  (Variables|Default|SetAttack%20Timer (- (Variables|Default|GetAttack%20Timer) DeltaSeconds)))

(fn ConstructionScript)