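; BP_MaurSuger is a ranged enemy that turns toward the astronaut and shoots rock projectiles at it.
; On BeginPlay it stores the astronaut as Target, found directly or through the possessed droid.
; Pawn sensing of astronaut or droid triggers aiming at Target and spawning BP_RockProjectile, throttled by a one-second CanAttack cooldown.
; DamageThis reduces Health and destroys the actor at zero, while DamageTarget is an empty stub.
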(event OnSeePawn(PawnSensing)
  (params (Pawn :type Pawn%20Object%20Reference))
  ;[1 1 1] Enemy Can Deal Damage
  (Utilities|Casting|CastToBP_Astronaut Pawn
    (:then
      _)
    (:CastFailed
      (Utilities|Casting|CastToBP_Droid Pawn)))
  (bind _returnvalue (CallFunction|GetTarget))
  (Transformation|SetActorRotation (Math|Rotator|FindLookatRotation (Transformation|GetActorLocation) (Transformation|GetActorLocation _returnvalue)))
  (if (Variables|Default|GetCanAttack)
    (Game|SpawnActorfromClass "/Game/Group_11/Blueprints/BP_RockProjectile.BP_RockProjectile_C" (Transformation|GetWorldTransform (Variables|Default|GetSpawnProjectileLocation)) "Undefined" "MultiplyWithRoot" 0 0)
    (Variables|Default|SetCanAttack false)
    (Utilities|FlowControl|Delay 1.0)
    (Variables|Default|SetCanAttack true)))

(event Custom|Dead
  ;[1 1 1] Added Death Event
  (Actor|DestroyActor))

(event EventDamageThis
  (params (DamageTaken :type Float%20%28single-precision%29))
  ;[1 1 1] Makes MaurSuger take damage
  (if (<= (Variables|Default|GetHealth) 0.0)
    (CallFunction|Dead)
    (else
      (bind _output_get (Variables|Default|SetHealth (- (Variables|Default|GetHealth) DamageTaken)))
      (if (<= _output_get 0.0)
        (CallFunction|Dead)))))

(event EventBeginPlay
  (bind _returnvalue (Game|Player|GetPlayerPawn 0))
  ;[1 1 1] Sets Target to Player
  (bind _asbp_astronaut (Utilities|Casting|CastToBP_Astronaut _returnvalue)
    (:then
      (CallFunction|SetTarget _asbp_astronaut))
    (:CastFailed
      (bind _asbp_droid (Utilities|Casting|CastToBP_Droid _returnvalue))
      (bind _returnvalue_2 (Class|Switch|GetAstronaut _asbp_droid))
      (bind _asbp_astronaut_2 (Utilities|Casting|CastToBP_Astronaut _returnvalue_2))
      (CallFunction|SetTarget _asbp_astronaut_2))))

(fn ConstructionScript)

(fn DamageTarget
  (params (DamageDealt :type Float%20%28single-precision%29))
  (return 0.0))

(fn GetTarget
  (return (Variables|Default|Gettarget)))

(fn SetTarget
  (params (newTarget :type Astronaut%20Object%20Reference))
  (bind _output_get (Variables|Default|Settarget newTarget))
  (Utilities|Casting|CastToBP_Astronaut _output_get
    (:then
      (return true))
    (:CastFailed
      (return false))))